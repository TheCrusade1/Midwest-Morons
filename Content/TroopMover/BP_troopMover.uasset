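; Troop-moving Blueprint that sends a group of AI troops to the spot a camera is looking at.
; The moveToCamera event casts each troop to Pawn and line traces forward from the camera against WorldDynamic objects only.
; Each pawn gets an AIMoveTo toward the hit location, without checking that the trace hit anything.
; Debug prints report the AIMoveTo output and any failed casts.
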(event `moveToCamera`
  (params (troops :type "Array of Actor Object Reference") (camera :type "/Game/Camera3/BP_CameraPawn3 Object Reference"))
  (bind _camera (`/Game/Camera3/BP_CameraPawn3.Camera` camera))
  (bind _returnvalue (`SceneComponent.K2_GetComponentLocation` _camera))
  (for _array_element troops
    (bind _aspawn (cast `Pawn` _array_element)
      (:`then`
        (bind _outhit (`KismetSystemLibrary.LineTraceSingleForObjects` _returnvalue (+ _returnvalue (* (`SceneComponent.GetForwardVector` _camera) 2500.0)) (`|MakeArray` "ObjectTypeQuery2" :!type "EObjectTypeQuery Enum")))
        (bind _movementresult (`|AIMoveTo` _aspawn (`.Location` (`GameplayStatics.BreakHitResult` _outhit)) null 100.0)
          (:`then`
            (`KismetSystemLibrary.PrintString` (`|GetEnumeratorNameAsString` _movementresult)))))
      (:`CastFailed`
        (`KismetSystemLibrary.PrintString` "troop failed to cast to pawn")))))

(fn `UserConstructionScript`)